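; BP_Tunnel is an endless-tunnel segment with a rotating holed wall, health pickup and shootable enemy.
; Passing TriggerZone scores a point; hitting the wall damages BP_Player, and either replaces the segment through TunnelSpawner unless the player dies.
; The pickup heals, enemy contact damages, and projectiles hitting HitBox destroy the enemy for a point.
; Randomize functions, not called here, vary wall mesh and roll plus pickup and enemy offsets.
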(event `self.ReceiveBeginPlay`
  (`self.PlayerRef`))

(event `PlayerRef`
  (bind _outactors (`GameplayStatics.GetAllActorsOfClass` "/Game/InfiniteMatrix/Blueprints/BP_Player.BP_Player_C"))
  (set `self.Player` (`|GetArrayItem` _outactors)))

(event `self.ReceiveTick`
  (params (DeltaSeconds :type "Float (single-precision)"))
  (`SceneComponent.K2_AddLocalRotation` (`self.WallMesh`) (`KismetMathLibrary.MakeRotator` (* DeltaSeconds (`self.RotateSpeed`))) false false))

(event `self.TriggerZone.OnComponentBeginOverlap`
  (params (OverlappedComponent :type "PrimitiveComponent Object Reference") (OtherActor :type "Actor Object Reference") (OtherComp :type "PrimitiveComponent Object Reference") (OtherBodyIndex :type Integer) (bFromSweep :type Boolean) (SweepResult :type "HitResult Structure (by ref)"))
  (bind _asbp_player (cast `/Game/InfiniteMatrix/Blueprints/BP_Player` OtherActor))
  (bind _output_get (set `/Game/InfiniteMatrix/Blueprints/BP_Player.Score` (+ (`/Game/InfiniteMatrix/Blueprints/BP_Player.Score` _asbp_player) 1) _asbp_player))
  (`/Game/InfiniteMatrix/Blueprints/BP_TunnelSpawner.SpawnTunnelAtSpawnPoint` (`self.TunnelSpawner`))
  (`self.K2_DestroyActor`)
  (`/Engine/EditorBlueprintResources/StandardMacros.IsValid` (`self.HealthPack`)
    (:`Is Valid`
      (`ActorComponent.K2_DestroyComponent` (`self.HealthPack`)))))

(event `self.WallMesh.OnComponentBeginOverlap`
  (params (OverlappedComponent :type "PrimitiveComponent Object Reference") (OtherActor :type "Actor Object Reference") (OtherComp :type "PrimitiveComponent Object Reference") (OtherBodyIndex :type Integer) (bFromSweep :type Boolean) (SweepResult :type "HitResult Structure (by ref)"))
  (bind _asbp_player (cast `/Game/InfiniteMatrix/Blueprints/BP_Player` OtherActor)
    (:`then`
      (`GameplayStatics.PlaySound2D` "/Game/Interface_And_Item_Sounds/WAV/Error_Buzz_05.Error_Buzz_05" 1.0 1.0 0.0 null null)
      (bind _output_get (set `/Game/InfiniteMatrix/Blueprints/BP_Player.HP` (`KismetMathLibrary.FClamp` (- (`/Game/InfiniteMatrix/Blueprints/BP_Player.HP` _asbp_player) 10.0) 0.0 100.0) _asbp_player))
      (`KismetSystemLibrary.PrintString` (`KismetStringLibrary.Conv_DoubleToString` _output_get))
      (if (== _output_get 0.0)
        (set `/Game/InfiniteMatrix/Blueprints/BP_Player.IsDead` true _asbp_player)
        (`/Game/InfiniteMatrix/Blueprints/BP_Player.DisplayRestart` _asbp_player)
        (else
          (`self.K2_DestroyActor`)
          (bind _asbp_tunnel_spawner (cast `/Game/InfiniteMatrix/Blueprints/BP_TunnelSpawner` (`self.TunnelSpawner`)))
          (`/Game/InfiniteMatrix/Blueprints/BP_TunnelSpawner.SpawnTunnelAtSpawnPoint` _asbp_tunnel_spawner))))
    (:`CastFailed`
      (bind _asbp_projectile (cast `/Game/InfiniteMatrix/Blueprints/BP_Projectile` OtherActor))
      (`self.K2_DestroyActor` _asbp_projectile))))

(event `self.HealthPack.OnComponentHit`
  (params (HitComponent :type "PrimitiveComponent Object Reference") (OtherActor :type "Actor Object Reference") (OtherComp :type "PrimitiveComponent Object Reference") (NormalImpulse :type "Vector Structure") (Hit :type "HitResult Structure (by ref)"))
  (bind _asbp_player (cast `/Game/InfiniteMatrix/Blueprints/BP_Player` OtherActor))
  (`GameplayStatics.PlaySound2D` "/Game/Interface_And_Item_Sounds/WAV/Special_Powerup_03.Special_Powerup_03" 1.0 1.0 0.0 null null)
  (bind _output_get (set `/Game/InfiniteMatrix/Blueprints/BP_Player.HP` (`KismetMathLibrary.FClamp` (+ (`/Game/InfiniteMatrix/Blueprints/BP_Player.HP` _asbp_player) 10.0) 0.0 100.0) _asbp_player))
  (`KismetSystemLibrary.PrintString` (`KismetStringLibrary.Conv_DoubleToString` _output_get))
  (`ActorComponent.K2_DestroyComponent` (`self.HealthPack`)))

(event `self.Enemy.OnComponentHit`
  (params (HitComponent :type "PrimitiveComponent Object Reference") (OtherActor :type "Actor Object Reference") (OtherComp :type "PrimitiveComponent Object Reference") (NormalImpulse :type "Vector Structure") (Hit :type "HitResult Structure (by ref)"))
  (bind _asbp_player (cast `/Game/InfiniteMatrix/Blueprints/BP_Player` OtherActor))
  (`GameplayStatics.PlaySound2D` "/Game/Interface_And_Item_Sounds/WAV/Error_Buzz_02.Error_Buzz_02" 1.0 1.0 0.0 null null)
  (bind _hp (`/Game/InfiniteMatrix/Blueprints/BP_Player.HP` _asbp_player))
  (if (== _hp 0.0)
    (`/Game/InfiniteMatrix/Blueprints/BP_Player.DisplayRestart` (`self.Player`))
    (else
      (set `/Game/InfiniteMatrix/Blueprints/BP_Player.HP` (`KismetMathLibrary.FClamp` (- _hp 10.0) 0.0 100.0) _asbp_player)
      (`KismetSystemLibrary.PrintString` "Player Collides with Ememy")
      (if (== (`/Game/InfiniteMatrix/Blueprints/BP_Player.HP` _asbp_player) 0.0)
        (`/Game/InfiniteMatrix/Blueprints/BP_Player.DisplayRestart` (`self.Player`))
        (`ActorComponent.K2_DestroyComponent` (`self.Enemy`))
        (else
          (`ActorComponent.K2_DestroyComponent` (`self.Enemy`)))))))

(event `self.HitBox.OnComponentBeginOverlap`
  (params (OverlappedComponent :type "PrimitiveComponent Object Reference") (OtherActor :type "Actor Object Reference") (OtherComp :type "PrimitiveComponent Object Reference") (OtherBodyIndex :type Integer) (bFromSweep :type Boolean) (SweepResult :type "HitResult Structure (by ref)"))
  (bind _enemy (`self.Enemy`))
  (bind _asbp_projectile (cast `/Game/InfiniteMatrix/Blueprints/BP_Projectile` OtherActor))
  (`GameplayStatics.SpawnEmitterAtLocation` "/Game/StarterContent/Particles/P_Explosion.P_Explosion" (`self.K2_GetActorLocation` _asbp_projectile) (struct) (4.0 4.0 4.0))
  (`GameplayStatics.PlaySound2D` "/Game/StarterContent/Audio/Explosion02.Explosion02" 1.0 1.0 0.0 null null)
  (`/Engine/EditorBlueprintResources/StandardMacros.IsValid` _enemy
    (:`Is Valid`
      (`ActorComponent.K2_DestroyComponent` _enemy)
      (`self.K2_DestroyActor` _asbp_projectile)
      (`ActorComponent.K2_DestroyComponent` (`self.HitBox`))
      (set `/Game/InfiniteMatrix/Blueprints/BP_Player.Score` (+ (`/Game/InfiniteMatrix/Blueprints/BP_Player.Score` (`self.Player`)) 1) (`self.Player`)))))

(fn `RandomizeEnemy`
  (`StaticMeshComponent.SetStaticMesh` (`self.Enemy`) "/Game/sA_PickupSet_1/Models/SM_Pickup_Magic.SM_Pickup_Magic")
  (`SceneComponent.K2_AddLocalOffset` (`self.Enemy`) (`KismetMathLibrary.MakeVector` (`KismetMathLibrary.RandomFloatInRange` -285.0 285.0) (`KismetMathLibrary.RandomFloatInRange` 500.0 2200.0) (`KismetMathLibrary.RandomFloatInRange` -285.0 285.0)) false false))

(fn `RandomizeHealthPack`
  (`StaticMeshComponent.SetStaticMesh` (`self.HealthPack`) "/Game/sA_PickupSet_1/Models/SM_Pickup_Health.SM_Pickup_Health")
  (`SceneComponent.K2_AddLocalOffset` (`self.HealthPack`) (`KismetMathLibrary.MakeVector` (`KismetMathLibrary.RandomFloatInRange` 500.0 2200.0) (`KismetMathLibrary.RandomFloatInRange` -285.0 285.0) (`KismetMathLibrary.RandomFloatInRange` -285.0 285.0)) false false))

(fn `RandomizeWall`
  (`StaticMeshComponent.SetStaticMesh` (`self.WallMesh`) (select `int` (`KismetMathLibrary.RandomIntegerInRange` 0 3) :`0` "/Game/InfiniteMatrix/Meshes/SM_Hole_01.SM_Hole_01" :`1` "/Game/InfiniteMatrix/Meshes/SM_Hole_02.SM_Hole_02" :`2` "/Game/InfiniteMatrix/Meshes/SM_Hole_03.SM_Hole_03" :`3` "/Game/InfiniteMatrix/Meshes/SM_Hole_04.SM_Hole_04" :!type "StaticMesh Object Reference"))
  (`SceneComponent.K2_AddLocalRotation` (`self.WallMesh`) (`KismetMathLibrary.MakeRotator` (`KismetMathLibrary.RandomFloatInRange` 0.0 360.0)) false false))

(fn `UserConstructionScript`)